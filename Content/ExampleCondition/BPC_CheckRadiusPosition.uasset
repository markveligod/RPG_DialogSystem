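; BPC_CheckRadiusPosition is an example condition that tests whether the player's controlled pawn is within a radius of a target point.
; It overrides IsConditionNative, validating the player controller, its pawn and the TargetPoint actor before comparing their distance to Radius.
; Any invalid reference makes the condition return false, and the Actor parameter goes unused.
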(fn `IsConditionNative`
  (params (PC :type "PlayerController Object Reference") (Actor :type "Actor Object Reference"))
  (returns (ReturnValue :type Boolean))
  (`/Engine/EditorBlueprintResources/StandardMacros.IsValid` (`local.PC`)
    (:`Is Valid`
      (`/Engine/EditorBlueprintResources/StandardMacros.IsValid` (`Controller.K2_GetPawn` (`local.PC`))
        (:`Is Valid`
          (`/Engine/EditorBlueprintResources/StandardMacros.IsValid` (`self.TargetPoint`)
            (:`Is Valid`
              (return (<= (`KismetMathLibrary.Vector_Distance` (`Actor.K2_GetActorLocation` (`self.TargetPoint`)) (`Actor.K2_GetActorLocation` (`Controller.K2_GetPawn` (`local.PC`)))) (`self.Radius`))))
            (:`Is Not Valid`
              _)))
        (:`Is Not Valid`
          _)))
    (:`Is Not Valid`
      _))
  (return false))