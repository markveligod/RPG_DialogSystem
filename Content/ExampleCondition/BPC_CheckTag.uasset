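; BPC_CheckTag is a condition that tests whether an actor carries a given gameplay tag name.
; Its IsConditionNative override checks the passed PC's Tags array when CheckSelf is set, otherwise the configured CheckActor's Tags.
; It returns false when the PC or the chosen CheckActor is invalid.
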(fn `IsConditionNative`
  (params (PC :type "PlayerController Object Reference") (Actor :type "Actor Object Reference"))
  (returns (ReturnValue :type Boolean))
  (`/Engine/EditorBlueprintResources/StandardMacros.IsValid` PC
    (:`Is Valid`
      (if (`self.CheckSelf?`)
        (return (`KismetArrayLibrary.Array_Contains` (`Actor.Tags` (`local.PC`)) (`self.CheckTag`)))
        (else
          (`/Engine/EditorBlueprintResources/StandardMacros.IsValid` (`self.CheckActor`)
            (:`Is Valid`
              (return (`KismetArrayLibrary.Array_Contains` (`Actor.Tags` (`self.CheckActor`)) (`self.CheckTag`))))
            (:`Is Not Valid`
              (return false))))))
    (:`Is Not Valid`
      (return false))))