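; BP_HUDTest is a HUD Blueprint that opens and closes the dialog UI for the owning player.
; RunDialog creates a WBP_Dialog only when none is active, adds it to the viewport and initializes it with the dialog object fetched from the passed actor.
; CompleteDialog removes the widget and clears the reference, so a new dialog can start.
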(event `DialogActionInterface.RunDialog`
  (params (ActorRunDialog :type "Actor Object Reference"))
  (`/Engine/EditorBlueprintResources/StandardMacros.IsValid` (`self.DialogWidget`)
    (:`Is Not Valid`
      (bind _returnvalue (`|CreateWidget` "/RPG_DialogSystem/WBP_Dialog.WBP_Dialog_C" (`self.GetOwningPlayerController`)))
      (`UserWidget.AddToViewport` _returnvalue 0)
      (bind _output_get (set `self.DialogWidget` _returnvalue))
      (bind _dialogobject (`RPG_DialogFunctionLibrary.GetDialogObject` ActorRunDialog))
      (`RPG_DialogWidget.InitWidget` _output_get _dialogobject))))

(event `DialogActionInterface.CompleteDialog`
  (params (ActorRunDialog :type "Actor Object Reference"))
  (`/Engine/EditorBlueprintResources/StandardMacros.IsValid` (`self.DialogWidget`)
    (:`Is Valid`
      (`Widget.RemoveFromParent` (`self.DialogWidget`))
      (set `self.DialogWidget` null))))

(fn `UserConstructionScript`)